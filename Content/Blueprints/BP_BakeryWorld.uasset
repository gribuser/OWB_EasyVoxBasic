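; BP_BakeryWorld generates a seeded procedural island terrain with OpenWorldBakery when play begins and displays it through its OWBEVWorldVisializer.
; BeginPlay sizes the bakery's heightmap from the visualizer's map resolution and splits it into a square grid of chunks.
; An asynchronous bake runs the terrain normal cycle on the big-island example hills setup, then creates the visualization once cooking completes.
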(event EventBeginPlay
  (bind _owb_ev_worldvisializer (Variables|Default|GetOWB_EV_WorldVisializer))
  (bind _openworldbakery (Variables|/Script/OWBEasyVoxel.OWB_EV_WorldVisializer|GetOpenWorldBakery _owb_ev_worldvisializer))
  (bind _mapresolution (Variables|/Script/OWBEasyVoxel.OWB_EV_WorldVisializer|GetMapResolution _owb_ev_worldvisializer))
  (bind _terrainseed (Variables|/Script/OWBEasyVoxel.OWB_EV_WorldVisializer|GetTerrainSeed _owb_ev_worldvisializer))
  (bind _returnvalue (/ _mapresolution 64))
  (Class|OWBHeightMapTerrainBase|InitHeightmap _openworldbakery (Utilities|Struct|MakeIntPoint _mapresolution _mapresolution))
  (Class|OWBCookedHeightMap|SetupChunks _openworldbakery _returnvalue _returnvalue)
  (|OpenWorldBake _openworldbakery (CallFunction|OWB:TerrainNormalCycle (CallFunction|OWB:ExampleHillsSetup:BigIsland _terrainseed) _terrainseed _openworldbakery)
    (:CookingComplete
      (Class|OWBEVWorldVisializer|CreateVisualization (Variables|Default|GetOWB_EV_WorldVisializer)))))

(event Collision|EventActorBeginOverlap
  (params (OtherActor :type Actor%20Object%20Reference)))

(event EventTick
  (params (DeltaSeconds :type Float%20%28single-precision%29)))

(fn ConstructionScript)